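; BP_SmithyGameInstance is the smithy game's game instance, holding the player's coffers and month number and persisting them through BP_SmithySaveGame.
; LoadGame creates a save object if needed, then restores both values from its slot when a save exists.
; SaveGame copies both values into the save object and writes it to that slot.
; ResetSave restores starting values and immediately saves them.
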(event `LoadGame`
  (bind _savefile (`self.SaveFile`))
  (bind _savefile_2 (`self.SaveFile`))
  (bind _savefile_3 (`self.SaveFile`))
  (`/Engine/EditorBlueprintResources/StandardMacros.IsValid` (`self.SaveFile`)
    (:`Is Valid`
      _)
    (:`Is Not Valid`
      (bind _returnvalue (`GameplayStatics.CreateSaveGameObject` "/Game/Blueprints/BP_SmithySaveGame.BP_SmithySaveGame_C"))
      (set `self.SaveFile` _returnvalue)))
  (bind _returnvalue_2 (`GameplayStatics.DoesSaveGameExist` (`/Game/Blueprints/BP_SmithySaveGame.SaveSlotName` _savefile) (`/Game/Blueprints/BP_SmithySaveGame.UserID` _savefile)))
  (if _returnvalue_2
    (bind _returnvalue_3 (`GameplayStatics.LoadGameFromSlot` (`/Game/Blueprints/BP_SmithySaveGame.SaveSlotName` _savefile_3) (`/Game/Blueprints/BP_SmithySaveGame.UserID` _savefile_3)))
    (set `self.SaveFile` (cast `/Game/Blueprints/BP_SmithySaveGame` _returnvalue_3 :!pure true))
    (set `self.MonthNumber` (`/Game/Blueprints/BP_SmithySaveGame.LastMonthFinished` _savefile_2))
    (set `self.Coffers` (`/Game/Blueprints/BP_SmithySaveGame.Coffers` _savefile_2))))

(event `SaveGame`
  (bind _savefile (`self.SaveFile`))
  (`/Engine/EditorBlueprintResources/StandardMacros.IsValid` (`self.SaveFile`)
    (:`Is Valid`
      _)
    (:`Is Not Valid`
      (bind _returnvalue (`GameplayStatics.CreateSaveGameObject` "/Game/Blueprints/BP_SmithySaveGame.BP_SmithySaveGame_C"))
      (set `self.SaveFile` _returnvalue)))
  (set `/Game/Blueprints/BP_SmithySaveGame.Coffers` (`self.Coffers`) _savefile)
  (set `/Game/Blueprints/BP_SmithySaveGame.LastMonthFinished` (`self.MonthNumber`) _savefile)
  (`GameplayStatics.SaveGameToSlot` _savefile (`/Game/Blueprints/BP_SmithySaveGame.SaveSlotName` _savefile) (`/Game/Blueprints/BP_SmithySaveGame.UserID` _savefile)))

(event `ResetSave`
  (set `self.Coffers` 0)
  (set `self.MonthNumber` 1)
  (`self.SaveGame`))