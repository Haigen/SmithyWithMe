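; BP_Item_IronShield is an iron shield item blueprint that extends a parent class.
; Its construction script creates a dynamic instance of the Ingot material on the item mesh and tints it a dark slate blue through the Colour parameter.
; Each tick, after calling the parent, it shows or hides its point light according to the IsSharp flag.
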(event `self.ReceiveTick`
  (params (DeltaSeconds :type "Float (single-precision)"))
  (`parent.ReceiveTick` DeltaSeconds)
  (`SceneComponent.SetVisibility` (`self.PointLight`) (`self.isSharp`) false))

(fn `UserConstructionScript`
  (`parent.UserConstructionScript`)
  (bind _returnvalue (`PrimitiveComponent.CreateDynamicMaterialInstance` (`self.ItemMesh`) 0 "/Game/Assets/Materials/Ingot.Ingot" "None"))
  (`MaterialInstanceDynamic.SetVectorParameterValue` _returnvalue "Colour" (struct :`R` 0.184475 :`G` 0.219526 :`B` 0.40724 :`A` 1.0)))