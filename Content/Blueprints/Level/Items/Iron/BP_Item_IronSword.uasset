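; BP_Item_IronSword is an iron sword item that builds on a parent Blueprint and shows a light while it is sharp.
; The construction script creates a dynamic instance of the shared Polyart item material on the item mesh and sets its material-type texture to iron.
; Tick runs the parent logic, then matches the point light's visibility to IsSharp every frame.
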(event `self.ReceiveTick`
  (params (DeltaSeconds :type "Float (single-precision)"))
  (`parent.ReceiveTick` DeltaSeconds)
  (`SceneComponent.SetVisibility` (`self.PointLight`) (`self.isSharp`) false))

(fn `UserConstructionScript`
  (`parent.UserConstructionScript`)
  (bind _returnvalue (`PrimitiveComponent.CreateDynamicMaterialInstance` (`self.ItemMesh`) 0 "/Game/Assets/ModularRPGHeroesPolyart/Materials/PolyartMatItems.PolyartMatItems" "None"))
  (`MaterialInstanceDynamic.SetTextureParameterValue` _returnvalue "MaterialType" "/Game/Assets/ModularRPGHeroesPolyart/Textures/PolyArtTexIron.PolyArtTexIron"))