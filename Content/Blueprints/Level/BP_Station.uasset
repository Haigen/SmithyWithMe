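; BP_Station is a crafting station that holds one item and converts it through repeated player interactions.
; PickUpDropFunction moves items between player and station, calling an empty CombineItemFunction when an accepted item arrives at an occupied station.
; Each interaction on an accepted item adds progress, plays audio and briefly shows a craft or forge progress bar.
; At full progress, ItemFinished replaces the item with the class returned by its Transform using AvailableRecipes.
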(event `self.ReceiveBeginPlay`
  (set `AudioComponent.Sound` (`self.InteractionSound`) (`self.Audio`)))

(event `self.ReceiveTick`
  (params (DeltaSeconds :type "Float (single-precision)"))
  (bind _curprogress (`self.CurProgress`))
  (bind _returnvalue (`WidgetComponent.GetUserWidgetObject` (`self.Progress`)))
  (bind _returnvalue_2 (select `bool` (== _curprogress 0.0) :`false` (/ _curprogress (`self.NeededProgress`)) :`true` 0.0))
  (bind _aswbp_progress_bar_craft (cast `/Game/Blueprints/UI/WBP_ProgressBarCraft` _returnvalue)
    (:`then`
      (set `/Game/Blueprints/UI/WBP_ProgressBarCraft.Percentage` _returnvalue_2 _aswbp_progress_bar_craft))
    (:`CastFailed`
      (bind _aswbp_progress_bar_forge (cast `/Game/Blueprints/UI/WBP_ProgressBarForge` _returnvalue))
      (set `/Game/Blueprints/UI/WBP_ProgressBarForge.Percentage` _returnvalue_2 _aswbp_progress_bar_forge))))

(event `InteractionEvent`
  (bind _storeditem (`self.StoredItem`))
  (`/Engine/EditorBlueprintResources/StandardMacros.IsValid` _storeditem
    (:`Is Valid`
      (if (`KismetArrayLibrary.Array_Contains` (`self.AcceptedItems`) (`GameplayStatics.GetObjectClass` _storeditem))
        (set `self.CurProgress` (+ (`self.CurProgress`) 20.0))
        (`SceneComponent.SetVisibility` (`self.Progress`) true false)
        (`|ExecutionSequence`
          (:`then_0`
            (if (>= (`self.CurProgress`) (`self.NeededProgress`))
              (set `self.CurProgress` 0.0)
              (`SceneComponent.SetVisibility` (`self.Progress`) false false)
              (`self.ItemFinished`)))
          (:`then_1`
            (`AudioComponent.Play` (`self.Audio`) 0.0))
          (:`then_2`
            (`KismetSystemLibrary.RetriggerableDelay` (`self.VanishTimer`))
            (`SceneComponent.SetVisibility` (`self.Progress`) false false)))))))

(fn `CombineItemFunction`
  (params (IncomingItem :type "/Game/Blueprints/Level/BP_Item Object Reference")))

(fn `ItemFinished`
  (bind _output_get (set `self.OldItem` (`self.StoredItem`)))
  (bind _itemtogive (`/Game/Blueprints/Level/BP_Item.Transform` _output_get (`self.AvailableRecipes`)))
  (bind _returnvalue (`|SpawnActorFromClass` _itemtogive (`SceneComponent.K2_GetComponentToWorld` (`self.ItemLocation`)) "AlwaysSpawn" "OverrideRootScale" null null))
  (bind _output_get_2 (set `self.StoredItem` _returnvalue))
  (`self.K2_DestroyActor` (`self.OldItem`))
  (`self.K2_AttachToComponent` _output_get_2 (`self.ItemLocation`) "None" "SnapToTarget" "SnapToTarget" "KeepRelative" true))

(fn `PickUpDropFunction`
  (params (IncomingItem :type "/Game/Blueprints/Level/BP_Item Object Reference") (CallingPlayer :type "/Game/Blueprints/Player/BP_Character Object Reference"))
  (bind _storeditem (`self.StoredItem`))
  (`/Engine/EditorBlueprintResources/StandardMacros.IsValid` IncomingItem
    (:`Is Valid`
      (if (or (`KismetArrayLibrary.Array_Contains` (`self.AcceptedItems`) (`GameplayStatics.GetObjectClass` IncomingItem)) (`self.AcceptAll`))
        ;[1 1 1] Store Item
        (`/Engine/EditorBlueprintResources/StandardMacros.IsValid` (`self.StoredItem`)
          (:`Is Valid`
            ;[1 1 1] Combining!
            (`self.CombineItemFunction` IncomingItem))
          (:`Is Not Valid`
            (`self.K2_DetachFromActor` IncomingItem "KeepWorld" "KeepWorld" "KeepWorld")
            (bind _output_get (set `self.StoredItem` IncomingItem))
            (set `/Game/Blueprints/Player/BP_Character.HeldItem` null CallingPlayer)
            (`self.K2_AttachToComponent` _output_get (`self.ItemLocation`) "None" "SnapToTarget" "SnapToTarget" "KeepWorld" true)))))
    (:`Is Not Valid`
      ;[1 1 1] Give Item To Player
      (`/Engine/EditorBlueprintResources/StandardMacros.IsValid` (`/Game/Blueprints/Player/BP_Character.HeldItem` CallingPlayer)
        (:`Is Not Valid`
          (`/Engine/EditorBlueprintResources/StandardMacros.IsValid` _storeditem
            (:`Is Valid`
              (`self.K2_DetachFromActor` _storeditem "KeepWorld" "KeepWorld" "KeepWorld")
              (bind _output_get_2 (set `/Game/Blueprints/Player/BP_Character.HeldItem` (`self.StoredItem`) CallingPlayer))
              (`self.K2_AttachToComponent` _output_get_2 (`/Game/Blueprints/Player/BP_Character.ItemPosition` CallingPlayer) "None" "SnapToTarget" "SnapToTarget" "KeepWorld" true)
              (set `self.StoredItem` null)
              (set `self.CurProgress` 0.0)
              (`SceneComponent.SetVisibility` (`self.Progress`) false false))))))))

(fn `UserConstructionScript`)