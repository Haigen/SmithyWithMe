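; BP_LobbyActor is a lobby player slot that displays a character and its joined state.
; The construction script uses ActorID to pick the Engineer or Elite skeletal mesh and a matching static mesh.
; On BeginPlay, UpdateJoinInfo toggles the particles and both meshes by Joined, then passes Joined and ActorID, as PlayerID, to the WBP_JoinButton in its widget component.
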(event `self.ReceiveBeginPlay`
  (`self.UpdateJoinInfo`))

(event `UpdateJoinInfo`
  (bind _joined (`self.Joined`))
  (bind _aswbp_join_button (cast `/Game/Blueprints/UI/WBP_JoinButton` (`WidgetComponent.GetUserWidgetObject` (`self.Widget`)) :!pure true))
  (`ActorComponent.SetActive` (`self.ParticleSystem`) _joined false)
  (`SceneComponent.SetVisibility` (`self.SkeletalMesh`) _joined true)
  (`SceneComponent.SetVisibility` (`self.StaticMesh1`) _joined true)
  (set `/Game/Blueprints/UI/WBP_JoinButton.HasJoined` (`self.Joined`) _aswbp_join_button)
  (set `/Game/Blueprints/UI/WBP_JoinButton.PlayerID` (`self.ActorID`) _aswbp_join_button))

(fn `UserConstructionScript`
  (`SkinnedMeshComponent.SetSkinnedAssetAndUpdate` (`self.SkeletalMesh`) (select `int` (`self.ActorID`) :`0` "/Game/Assets/ModularRPGHeroesPolyart/Meshes/OneMeshCharacters/EngineerSK.EngineerSK" :`1` "/Game/Assets/ModularRPGHeroesPolyart/Meshes/OneMeshCharacters/EliteSK.EliteSK" :!type "SkeletalMesh Object Reference") true)
  (`StaticMeshComponent.SetStaticMesh` (`self.StaticMesh1`) (select `int` (`self.ActorID`) :`0` "/Game/Assets/Models/HotShape.HotShape" :`1` "/Game/Assets/Models/HotShapeShield.HotShapeShield" :!type "StaticMesh Object Reference")))