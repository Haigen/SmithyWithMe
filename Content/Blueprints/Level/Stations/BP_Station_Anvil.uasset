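; Anvil crafting station Blueprint, a child of a station parent class that players interact with.
; On interaction it picks one of two random impact sounds for the audio component, then runs the parent interaction logic.
; If the stored item's class is in the accepted items, it spawns scaled hammer spark particles at the particle location component.
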(event `self.InteractionEvent`
  (params (PlayerID :type Integer))
  (bind _storeditem (`self.StoredItem`))
  (bind _output_get (set `self.InteractionSound` (select `int` (`KismetMathLibrary.RandomInteger` 2) :`0` "/Game/Assets/autumnbs/Audio/Anvil/CUE/Anvil_Impact_01.Anvil_Impact_01" :`1` "/Game/Assets/autumnbs/Audio/Anvil/CUE/Anvil_Impact_02.Anvil_Impact_02" :!type "SoundCue Object Reference")))
  (set `AudioComponent.Sound` _output_get (`self.Audio`))
  (`parent.InteractionEvent` PlayerID)
  (`/Engine/EditorBlueprintResources/StandardMacros.IsValid` _storeditem
    (:`Is Valid`
      (if (`KismetArrayLibrary.Array_Contains` (`self.AcceptedItems`) (`GameplayStatics.GetObjectClass` _storeditem))
        (`GameplayStatics.SpawnEmitterAtLocation` "/Game/Assets/InfinityBladeEffects/Effects/FX_Forging/P_HammerSparks.P_HammerSparks" (`SceneComponent.K2_GetComponentLocation` (`self.ParticleLoc`)) (struct) (2.5 2.5 2.5))))))

(fn `UserConstructionScript`
  (`parent.UserConstructionScript`))