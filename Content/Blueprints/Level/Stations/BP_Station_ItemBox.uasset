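; BP_Station_ItemBox is a station that dispenses a limited stock of one ore type to players.
; PickUpDropFunction spawns the ItemType's item for an empty-handed player, attaches it to their ItemPosition, decrements ItemCount and plays a sound.
; The construction script tints the contents mesh through a dynamic material, and a text label showing the count refreshes every Tick.
; Only copper, iron and steel ores have item classes and colours assigned.
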(event `self.ReceiveTick`
  (params (DeltaSeconds :type "Float (single-precision)"))
  (`parent.ReceiveTick` DeltaSeconds)
  (`TextRenderComponent.K2_SetText` (`self.TextRender`) (`KismetTextLibrary.Conv_IntToText` (`self.ItemCount`))))

(event `self.PickUpDropFunction`
  (params (IncomingItem :type "/Game/Blueprints/Level/BP_Item Object Reference") (CallingPlayer :type "/Game/Blueprints/Player/BP_Character Object Reference"))
  (if (> (`self.ItemCount`) 0)
    ;[1 1 1] Give Item To Player
    (`/Engine/EditorBlueprintResources/StandardMacros.IsValid` (`/Game/Blueprints/Player/BP_Character.HeldItem` CallingPlayer)
      (:`Is Not Valid`
        (bind _returnvalue (`|SpawnActorFromClass` (select `/Game/Blueprints/Level/Enum_ItemType` (`self.ItemType`) :`NewEnumerator0` "/Game/Blueprints/Level/Items/Copper/BP_Item_CopperOre.BP_Item_CopperOre_C" :`NewEnumerator1` "/Game/Blueprints/Level/Items/Iron/BP_Item_IronOre.BP_Item_IronOre_C" :`NewEnumerator2` "/Game/Blueprints/Level/Items/Steel/BP_Item_SteelOre.BP_Item_SteelOre_C" :!type "Actor Class Reference") (`SceneComponent.K2_GetComponentToWorld` (`self.ItemLocation`)) "Undefined" "OverrideRootScale" null null))
        (bind _output_get (set `/Game/Blueprints/Player/BP_Character.HeldItem` (cast `/Game/Blueprints/Level/BP_Item` _returnvalue :!pure true) CallingPlayer))
        (`self.K2_AttachToComponent` _output_get (`/Game/Blueprints/Player/BP_Character.ItemPosition` CallingPlayer) "None" "SnapToTarget" "SnapToTarget" "KeepWorld" true)
        (`/Engine/EditorBlueprintResources/StandardMacros.DecrementInt` (`self.ItemCount`)
          (:`  `
            (`GameplayStatics.PlaySoundAtLocation` self (`self.InteractionSound`) (`self.K2_GetActorLocation` self) (struct) 1.0 1.0 0.0 null null null)))))))

(fn `UserConstructionScript`
  (`parent.UserConstructionScript`)
  (bind _returnvalue (`PrimitiveComponent.CreateDynamicMaterialInstance` (`self.ItemContainMesh`) 0 "/Game/Assets/Materials/Ore.Ore" "None"))
  (`MaterialInstanceDynamic.SetVectorParameterValue` _returnvalue "Colour" (select `/Game/Blueprints/Level/Enum_ItemType` (`self.ItemType`) :`NewEnumerator0` (struct :`R` 0.300544 :`G` 0.14996 :`A` 1.0) :`NewEnumerator1` (struct :`R` 0.184475 :`G` 0.219526 :`B` 0.40724 :`A` 1.0) :`NewEnumerator2` (struct :`R` 0.467784 :`G` 0.467784 :`B` 0.467784 :`A` 1.0) :!type "LinearColor Structure"))
  (`TextRenderComponent.K2_SetText` (`self.TextRender`) (`KismetTextLibrary.Conv_IntToText` (`self.ItemCount`))))