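; Sell box station that turns a player's held item into earnings when the pick up/drop interaction fires.
; It clears the held item, spawns a money particle, then looks up the item's cost in a data table by type name.
; A found row destroys the item, adds its cost to game mode Earnings and plays a sound.
; The in-demand type, kept current through a game mode event binding, pays a rounded 1.5x.
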(event `self.ReceiveBeginPlay`
  (`parent.ReceiveBeginPlay`)
  (bind _asbp_working_game_mode (cast `/Game/Blueprints/BP_WorkingGameMode` (`GameplayStatics.GetGameMode`)))
  (add `/Game/Blueprints/BP_WorkingGameMode.UpdateInDemand` _asbp_working_game_mode (delegate `UpdateInDemand`)))

(event `UpdateInDemand`
  (params (ItemInDemand :type "/Game/Blueprints/Level/Data/Enum_ItemType Enum" :default "NewEnumerator0"))
  (set `self.InDemand` ItemInDemand))

(event `self.PickUpDropFunction`
  (params (IncomingItem :type "/Game/Blueprints/Level/BP_Item Object Reference") (CallingPlayer :type "/Game/Blueprints/Player/BP_Character Object Reference"))
  (bind _helditem (`/Game/Blueprints/Player/BP_Character.HeldItem` CallingPlayer))
  (bind (_itemtype _cost) (break `/Game/Blueprints/Level/Data/Struct_ItemsCosts` (`self.ItemCostGet`)))
  (bind _asbp_working_game_mode (cast `/Game/Blueprints/BP_WorkingGameMode` (`GameplayStatics.GetGameMode`) :!pure true))
  ;[1 1 1] Sell
  (`/Engine/EditorBlueprintResources/StandardMacros.IsValid` _helditem
    (:`Is Valid`
      (set `self.ItemToDel` _helditem)
      (set `/Game/Blueprints/Player/BP_Character.HeldItem` null CallingPlayer)
      (`GameplayStatics.SpawnEmitterAtLocation` "/Game/Assets/Particles/MoneyParticle.MoneyParticle" (`SceneComponent.K2_GetComponentLocation` (`self.ParticleLoc`)))
      (bind _returnvalue (`|GetDataTableRow` (`self.CostDataTable`) (`KismetStringLibrary.Conv_StringToName` (`|GetEnumeratorNameAsString` (`/Game/Blueprints/Level/BP_Item.MyType` (`self.ItemToDel`)))))
        (:`then`
          (set `self.ItemCostGet` _returnvalue)
          (`self.K2_DestroyActor` (`self.ItemToDel`))
          (set `/Game/Blueprints/BP_WorkingGameMode.Earnings` (+ (`/Game/Blueprints/BP_WorkingGameMode.Earnings` _asbp_working_game_mode) (select `bool` (== _itemtype (`self.InDemand`)) :`false` _cost :`true` (`KismetMathLibrary.Round` (* _cost 1.5)))) _asbp_working_game_mode)
          (`GameplayStatics.PlaySoundAtLocation` self (`self.InteractionSound`) (`self.K2_GetActorLocation` self) (struct) 1.0 1.0 0.0 null null null)
          (set `self.ItemCostGet` (struct)))))))

(fn `UserConstructionScript`
  (`parent.UserConstructionScript`))