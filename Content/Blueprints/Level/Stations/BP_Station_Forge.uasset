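; Forge station that automatically processes an accepted stored item over time, using inherited station logic.
; Each Tick, AutoProgress advances progress with sound, particles and a progress display, then calls ItemFinished at the threshold.
; Without a valid item it stops the effects and clears progress.
; Interacting with the accepted tool (bellows) adds a fifth of the needed progress.
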(event `self.ReceiveTick`
  (params (DeltaSeconds :type "Float (single-precision)"))
  (bind _storeditem (`self.StoredItem`))
  (`parent.ReceiveTick` DeltaSeconds)
  (if (and (`KismetSystemLibrary.IsValid` _storeditem) (`KismetArrayLibrary.Array_Contains` (`self.AcceptedItems`) (`GameplayStatics.GetObjectClass` _storeditem)))
    (`|ExecutionSequence`
      (:`then_0`
        (`/Engine/EditorBlueprintResources/StandardMacros.DoOnce` false :!label _label
          (:`Completed`
            (`self.StartSound`))))
      (:`then_1`
        (if (not (`ActorComponent.IsActive` (`self.ParticleSystem`)))
          (`ActorComponent.Activate` (`self.ParticleSystem`) true))
        (`SceneComponent.SetVisibility` (`self.Progress`) true false)
        (bind _output_get (set `self.CurProgress` (+ (`self.CurProgress`) DeltaSeconds)))
        (if (>= _output_get (`self.NeededProgress`))
          (set `self.CurProgress` 0.0)
          (`self.ItemFinished`)
          (goto _label :!via `Reset`))))
    (else
      (`|ExecutionSequence`
        (:`then_0`
          (`self.StopSound`))
        (:`then_1`
          (`ActorComponent.Deactivate` (`self.ParticleSystem`))
          (`SceneComponent.SetVisibility` (`self.Progress`) false false)
          (set `self.CurProgress` 0.0))))))

(event `StartSound`
  (`AudioComponent.Play` (`self.Audio`) 0.0))

(event `StopSound`
  (`AudioComponent.Stop` (`self.Audio`)))

(event `self.InteractionEvent`
  (params (PlayerID :type Integer))
  (bind _storeditem (`self.StoredItem`))
  ;[1 1 1] Do nothing unless, player is holding bellows
  (if (and (`KismetSystemLibrary.IsValid` _storeditem) (`KismetArrayLibrary.Array_Contains` (`self.AcceptedItems`) (`GameplayStatics.GetObjectClass` _storeditem)) (`|EnumEquality` (`/Game/Blueprints/Player/BP_Character.ToolType` (cast `/Game/Blueprints/Player/BP_Character` (`GameplayStatics.GetPlayerCharacter` PlayerID) :!pure true)) (`self.AcceptedInteractionTool`)))
    (set `self.CurProgress` (+ (`self.CurProgress`) (/ (`self.NeededProgress`) 5.0)))))

(fn `UserConstructionScript`
  (`parent.UserConstructionScript`))