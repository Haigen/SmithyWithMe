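; Grindstone crafting station that sharpens the item stored in it.
; Interactions pass to the parent station logic only while a valid, unsharpened item is stored, and each one spawns impact sparks at the particle marker.
; When the item finishes, it is flagged as sharp and its price is updated.
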(event `self.ItemFinished`
  (bind _storeditem (`self.StoredItem`))
  (set `/Game/Blueprints/Level/BP_Item.isSharp` true _storeditem)
  (`/Game/Blueprints/Level/BP_Item.UpdatePrice` _storeditem))

(event `self.InteractionEvent`
  (params (PlayerID :type Integer))
  (bind _storeditem (`self.StoredItem`))
  (bind _particleloc (`self.ParticleLoc`))
  (`/Engine/EditorBlueprintResources/StandardMacros.IsValid` _storeditem
    (:`Is Valid`
      (if (not (`/Game/Blueprints/Level/BP_Item.isSharp` _storeditem))
        (`parent.InteractionEvent` PlayerID)
        (`GameplayStatics.SpawnEmitterAtLocation` "/Game/Assets/InfinityBladeEffects/Effects/FX_Combat_Base/Impact/P_ImpactSparks.P_ImpactSparks" (`SceneComponent.K2_GetComponentLocation` _particleloc) (`SceneComponent.K2_GetComponentRotation` _particleloc))))))

(fn `UserConstructionScript`
  (`parent.UserConstructionScript`))