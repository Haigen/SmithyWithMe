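; Game mode for the smithy game that runs one month per level load, from save loading to month-end accounting.
; BeginPlay restores state, fills item boxes, creates the HUD and trims extra characters in single-player, then starts looping day and week timers.
; Weeks trigger demand changes; month end deducts month-scaled tax and material costs, then shows report and purchase screens.
; Continuing saves through the game instance and reloads; quitting resets the save.
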(event `self.ReceiveBeginPlay`
  (bind _output_get (set `self.GameInstance` (cast `/Game/Blueprints/BP_SmithyGameInstance` (`GameplayStatics.GetGameInstance`) :!pure true)))
  (`/Game/Blueprints/BP_SmithyGameInstance.LoadGame` _output_get)
  (set `self.MonthNumber` (`/Game/Blueprints/BP_SmithyGameInstance.MonthNumber` _output_get))
  (set `self.Coffers` (`/Game/Blueprints/BP_SmithyGameInstance.Coffers` _output_get))
  (set `self.CopperOreCount` (`/Game/Blueprints/BP_SmithyGameInstance.CopperOreCount` _output_get))
  (set `self.IronOreCount` (`/Game/Blueprints/BP_SmithyGameInstance.IronOreCount` _output_get))
  (bind _outactors (`GameplayStatics.GetAllActorsOfClass` "/Game/Blueprints/Level/Stations/BP_Station_ItemBox.BP_Station_ItemBox_C"))
  (for _array_element _outactors
    (`/Game/Blueprints/Level/Stations/BP_Station_ItemBox.UpdateAmounts` _array_element (`self.CopperOreCount`) (`self.IronOreCount`)))
  (bind _returnvalue (`|CreateWidget` "/Game/Blueprints/UI/WBP_GameUI.WBP_GameUI_C" (`GameplayStatics.GetPlayerController` 0)))
  (bind _output_get_2 (set `self.GameUI` _returnvalue))
  (`UserWidget.AddToPlayerScreen` _output_get_2 1)
  (set `/Game/Blueprints/UI/WBP_GameUI.DayNum` (`self.DayNum`) (`self.GameUI`))
  (if (== (`/Game/Blueprints/BP_SmithyGameInstance.NumOfPlayers` (`self.GameInstance`)) 1)
    (bind _outactors_2 (`GameplayStatics.GetAllActorsOfClass` "/Game/Blueprints/Player/BP_Character.BP_Character_C"))
    (for _array_element_2 _outactors_2
      (if (!= _array_element_2 (`GameplayStatics.GetPlayerCharacter` 0))
        (`self.K2_DestroyActor` _array_element_2))))
  (`KismetSystemLibrary.Delay` 3.0) ; Wait to Start
  (bind _returnvalue_2 (`KismetSystemLibrary.K2_SetTimerDelegate` (delegate `NextDay`) (`self.DayLength`) true))
  (set `self.DayTimer` _returnvalue_2)
  (bind _returnvalue_3 (`KismetSystemLibrary.K2_SetTimerDelegate` (delegate `NewWeekEvent`) (* (`self.DayLength`) (`KismetMathLibrary.Conv_IntToDouble` (`self.WeekLength`))) true))
  (set `self.WeekTimer` _returnvalue_3))

(event `NewWeekEvent`
  (`self.HighDemandEvent`))

(event `NextDay`
  (set `self.DayNum` (+ (`self.DayNum`) 1))
  (if (> (`self.DayNum`) (`self.MonthLength`))
    (`self.UpdateEndScreen`)
    (`KismetSystemLibrary.K2_ClearAndInvalidateTimerHandle` (`self.DayTimer`))
    (else
      (set `/Game/Blueprints/UI/WBP_GameUI.DayNum` (`self.DayNum`) (`self.GameUI`))
      (`/Game/Blueprints/UI/WBP_GameUI.UpdateDay` (`self.GameUI`)))))

(event `self.ReceiveTick`
  (params (DeltaSeconds :type "Float (single-precision)"))
  (bind _gameui (`self.GameUI`))
  (set `/Game/Blueprints/UI/WBP_GameUI.Percentage` (/ (`KismetSystemLibrary.K2_GetTimerRemainingTimeHandle` (`self.DayTimer`)) (`self.DayLength`)) _gameui)
  (set `/Game/Blueprints/UI/WBP_GameUI.Earnings` (`self.Earnings`) _gameui)
  (set `/Game/Blueprints/UI/WBP_GameUI.WeekPercentage` (- 1.0 (/ (`KismetSystemLibrary.K2_GetTimerRemainingTimeHandle` (`self.WeekTimer`)) (* (`self.DayLength`) (`KismetMathLibrary.Conv_IntToDouble` (`self.WeekLength`))))) _gameui))

(event `UpdateEndScreen`
  (bind _reportscreen (`self.ReportScreen`))
  (bind _reportscreen_2 (`self.ReportScreen`))
  (bind _returnvalue (`KismetMathLibrary.Round` (`KismetMathLibrary.MultiplyMultiply_FloatFloat` (`KismetMathLibrary.Conv_IntToDouble` (`self.MonthNumber`)) 2.0)))
  (set `self.LandTaxCost` (/ (* 40 _returnvalue) 5))
  (set `self.MaterialsCost` (/ (* 30 _returnvalue) 5))
  (set `self.Coffers` (- (+ (`self.Coffers`) (`self.Earnings`)) (+ (`self.LandTaxCost`) (`self.MaterialsCost`))))
  (set `self.DayNum` 1)
  (set `self.GotGameOver` (<= (`self.Coffers`) 0))
  (set `/Game/Blueprints/Player/BP_Character.IsOnReportScreen` true (cast `/Game/Blueprints/Player/BP_Character` (`GameplayStatics.GetPlayerCharacter` 0) :!pure true))
  (bind _returnvalue_2 (`|CreateWidget` "/Game/Blueprints/UI/WBP_ReportScreen.WBP_ReportScreen_C" (`GameplayStatics.GetPlayerController` 0)))
  (bind _output_get (set `self.ReportScreen` _returnvalue_2))
  (`UserWidget.AddToPlayerScreen` _output_get 3)
  (set `PlayerController.bShowMouseCursor` true (`GameplayStatics.GetPlayerController` 0))
  (add `/Game/Blueprints/UI/WBP_ReportScreen.NextMenu` _reportscreen_2 (delegate `ShopMenu`))
  (add `/Game/Blueprints/UI/WBP_ReportScreen.QuitGame` _reportscreen_2 (delegate `Quit`))
  (set `/Game/Blueprints/UI/WBP_ReportScreen.Earnings` (`self.Earnings`) _reportscreen)
  (set `/Game/Blueprints/UI/WBP_ReportScreen.LandTax` (`self.LandTaxCost`) _reportscreen)
  (set `/Game/Blueprints/UI/WBP_ReportScreen.MaterialsCost` (`self.MaterialsCost`) _reportscreen)
  (set `/Game/Blueprints/UI/WBP_ReportScreen.Coffers` (`self.Coffers`) _reportscreen)
  (set `/Game/Blueprints/UI/WBP_ReportScreen.MonthNum` (`self.MonthNumber`) _reportscreen)
  (set `/Game/Blueprints/UI/WBP_ReportScreen.CanGoNext` (not (`self.GotGameOver`)) _reportscreen))

(event `ShopMenu`
  (bind _purchasescreen (`self.PurchaseScreen`))
  (bind _purchasescreen_2 (`self.PurchaseScreen`))
  (`Widget.RemoveFromParent` (`self.ReportScreen`))
  (bind _returnvalue (`|CreateWidget` "/Game/Blueprints/UI/WBP_PurchaseScreen.WBP_PurchaseScreen_C" (`GameplayStatics.GetPlayerController` 0)))
  (bind _output_get (set `self.PurchaseScreen` _returnvalue))
  (`UserWidget.AddToPlayerScreen` _output_get 0)
  (add `/Game/Blueprints/UI/WBP_PurchaseScreen.NextLevel` _purchasescreen_2 (delegate `NextMonth`))
  (add `/Game/Blueprints/UI/WBP_PurchaseScreen.QuitGame` _purchasescreen_2 (delegate `Quit`))
  (set `/Game/Blueprints/UI/WBP_PurchaseScreen.Coffers` (`self.Coffers`) _purchasescreen)
  (set `/Game/Blueprints/UI/WBP_PurchaseScreen.CopperOreCost` 0 _purchasescreen)
  (set `/Game/Blueprints/UI/WBP_PurchaseScreen.IronOreCost` 0 _purchasescreen))

(event `HighDemandEvent`
  (`self.UpdateInDemand` (select `int` (/ (`self.DayNum`) (`self.WeekLength`)) :`0` "NewEnumerator24" :`1` "NewEnumerator24" :`2` "NewEnumerator9" :`3` "NewEnumerator24" :`4` "NewEnumerator20" :`5` "NewEnumerator20" :`6` "NewEnumerator24" :!type "/Game/Blueprints/Level/Data/Enum_ItemType Enum")))

(event `Quit`
  (`/Game/Blueprints/BP_SmithyGameInstance.ResetSave` (cast `/Game/Blueprints/BP_SmithyGameInstance` (`GameplayStatics.GetGameInstance`) :!pure true))
  (`GameplayStatics.OpenLevel` "LVL_MainMenu"))

(event `NextMonth`
  (bind _asbp_smithy_game_instance (cast `/Game/Blueprints/BP_SmithyGameInstance` (`GameplayStatics.GetGameInstance`) :!pure true))
  (set `/Game/Blueprints/BP_SmithyGameInstance.Coffers` (`self.Coffers`) _asbp_smithy_game_instance)
  (set `/Game/Blueprints/BP_SmithyGameInstance.MonthNumber` (+ (`self.MonthNumber`) 1) _asbp_smithy_game_instance)
  (`/Game/Blueprints/BP_SmithyGameInstance.SaveGame` _asbp_smithy_game_instance)
  (`GameplayStatics.OpenLevel` "LVL_MainGame"))

(fn `UserConstructionScript`)