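; Player character for a smithy game that moves on world axes, carries items and works at stations with a hammer, bellows or tongs.
; Tick turns the mesh toward movement input and sphere-traces ahead to highlight the current BP_Station, which pickup and interact inputs act on.
; Tool selection swaps a child actor class.
; On the report screen, axis input fires DoOnce-gated menu calls instead of moving; debug-style Subtract key resets the save.
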(event `self.ReceiveBeginPlay`
  (`EnhancedInputSubsystemInterface.AddMappingContext` (pcsubsystem `EnhancedInputLocalPlayerSubsystem` (`GameplayStatics.GetPlayerController` 0)) "/Game/Blueprints/Input/IMC_Gameplay.IMC_Gameplay" 0 (struct)))

(event `EnhancedInput|/Game/Blueprints/Input/IA_Pickup`
  (params (ActionValue :type Boolean) (ElapsedSeconds :type "Float (double-precision)") (TriggeredSeconds :type "Float (double-precision)") (InputAction :type "InputAction Object Reference" :default "/Game/Blueprints/Input/IA_Pickup.IA_Pickup"))
  (bind _curstation (`self.CurStation`))
  (bind _helditem (`self.HeldItem`))
  (:`Started`
    (`/Engine/EditorBlueprintResources/StandardMacros.IsValid` _curstation
      (:`Is Valid`
        (`/Game/Blueprints/Level/BP_Station.PickUpDropFunction` _curstation _helditem self)
        (set `self.HasItem` (`KismetSystemLibrary.IsValid` _helditem))))))

(event `self.ReceiveTick`
  (params (DeltaSeconds :type "Float (single-precision)"))
  (bind _curstation (`self.CurStation`))
  (bind _curstation_2 (`self.CurStation`))
  (bind _reachpos (`self.ReachPos`))
  (bind _returnvalue (`SceneComponent.K2_GetComponentLocation` _reachpos))
  (`|ExecutionSequence`
    (:`then_0`
      (if (or (!= (`self.GetInputAxisValue`) 0.0) (!= (`self.GetInputAxisValue`) 0.0))
        (set `self.direction` (`KismetMathLibrary.MakeVector` (`self.GetInputAxisValue`) (`self.GetInputAxisValue`)))
        (`SceneComponent.K2_SetWorldRotation` (`self.Mesh`) (`KismetMathLibrary.RLerp` (`SceneComponent.K2_GetComponentRotation` (`self.Mesh`)) (`KismetMathLibrary.MakeRotator` (.roll (`KismetMathLibrary.Conv_VectorToRotator` (`self.direction`))) (.pitch (`KismetMathLibrary.Conv_VectorToRotator` (`self.direction`))) (+ (.yaw (`KismetMathLibrary.Conv_VectorToRotator` (`self.direction`))) -90.0)) (* DeltaSeconds (`self.RotationSpeed`)) true) false false)))
    (:`then_1`
      (bind (_outhit _returnvalue_2) (`KismetSystemLibrary.SphereTraceSingle` _returnvalue (+ _returnvalue (* (`SceneComponent.GetForwardVector` _reachpos) (`self.Reach`))) (`self.RadiusCheck`) "TraceTypeQuery1"))
      (if _returnvalue_2
        (`/Engine/EditorBlueprintResources/StandardMacros.IsValid` _curstation
          (:`Is Valid`
            (set `/Game/Blueprints/Level/BP_Station.Highlighted` false _curstation))
          (:`Is Not Valid`
            _))
        (bind _asbp_station (cast `/Game/Blueprints/Level/BP_Station` (`.HitActor` (`GameplayStatics.BreakHitResult` _outhit))))
        (bind _output_get (set `self.CurStation` _asbp_station))
        (set `/Game/Blueprints/Level/BP_Station.Highlighted` true _output_get)
        (else
          (`/Engine/EditorBlueprintResources/StandardMacros.IsValid` _curstation_2
            (:`Is Valid`
              (set `/Game/Blueprints/Level/BP_Station.Highlighted` false _curstation_2))
            (:`Is Not Valid`
              _))
          (set `self.CurStation` null))))))

(event `InputAction|CycleToolLeft`
  (params (Key :type "Key Structure"))
  (:`Pressed`
    (switch `/Game/Blueprints/Enums/Enum_ToolType` (`self.ToolType`)
      (:`NewEnumerator0`
        (set `self.ToolType` "NewEnumerator2" :!label _label))
      (:`NewEnumerator1`
        (set `self.ToolType` "NewEnumerator0" :!label _label_2))
      (:`NewEnumerator2`
        (set `self.ToolType` "NewEnumerator1" :!label _label_3)))
    (`self.UpdateTool`)))

(event `EnhancedInput|/Game/Blueprints/Input/IA_Interact`
  (params (ActionValue :type Boolean) (ElapsedSeconds :type "Float (double-precision)") (TriggeredSeconds :type "Float (double-precision)") (InputAction :type "InputAction Object Reference" :default "/Game/Blueprints/Input/IA_Interact.IA_Interact"))
  (bind _curstation (`self.CurStation`))
  (bind _storeditem (`/Game/Blueprints/Level/BP_Station.StoredItem` _curstation))
  (:`Triggered`
    (`/Engine/EditorBlueprintResources/StandardMacros.IsValid` (`self.CurStation`)
      (:`Is Valid`
        (if (and (`KismetSystemLibrary.IsValid` _storeditem) (`KismetArrayLibrary.Array_Contains` (`/Game/Blueprints/Level/BP_Station.AcceptedItems` _curstation) (`GameplayStatics.GetObjectClass` _storeditem)))
          (`/Game/Blueprints/Level/BP_Station.InteractionEvent` (`self.CurStation`) (`GameplayStatics.GetPlayerControllerID` (cast `/Game/Blueprints/Player/BP_CharacterController` (`self.GetController`) :!pure true)))
          (set `self.Working` true)
          (else
            (set `self.Working` false))))))
  (:`Canceled`
    (set `self.Working` false :!label _label_4))
  (:`Completed`
    (goto _label_4)))

(event `InputAction|CycleToolRight`
  (params (Key :type "Key Structure"))
  (:`Pressed`
    (switch `/Game/Blueprints/Enums/Enum_ToolType` (`self.ToolType`)
      (:`NewEnumerator0`
        (goto _label_3))
      (:`NewEnumerator1`
        (goto _label))
      (:`NewEnumerator2`
        (goto _label_2)))))

(event `Key|One`
  (params (Key :type "Key Structure"))
  (:`Pressed`
    (set `self.ToolType` "NewEnumerator0")
    (`self.UpdateTool` :!label _label_5)))

(event `Key|Subtract`
  (params (Key :type "Key Structure"))
  (:`Pressed`
    (`/Game/Blueprints/BP_SmithyGameInstance.ResetSave` (cast `/Game/Blueprints/BP_SmithyGameInstance` (`GameplayStatics.GetGameInstance`) :!pure true))))

(event `Key|Two`
  (params (Key :type "Key Structure"))
  (:`Pressed`
    (set `self.ToolType` "NewEnumerator1")
    (goto _label_5)))

(event `ShowToolTip`
  (params (ToolType :type "/Game/Blueprints/Enums/Enum_ToolType Enum" :default "NewEnumerator0") (isStation :type Boolean))
  (bind _widget (`self.Widget`))
  (set `self.ToolTipType` ToolType)
  (set `self.isStation` isStation)
  (`SceneComponent.SetVisibility` _widget true false)
  (`KismetSystemLibrary.RetriggerableDelay` 1.0)
  (`SceneComponent.SetVisibility` _widget false false))

(event `Key|Three`
  (params (Key :type "Key Structure"))
  (:`Pressed`
    (set `self.ToolType` "NewEnumerator2")
    (goto _label_5)))

(event `UpdateTool`
  (`ChildActorComponent.SetChildActorClass` (`self.ChildActor`) (select `/Game/Blueprints/Enums/Enum_ToolType` (`self.ToolType`) :`NewEnumerator0` "/Game/Blueprints/Player/Tools/BP_Tool_Hammer.BP_Tool_Hammer_C" :`NewEnumerator1` "/Game/Blueprints/Player/Tools/BP_Tool_Bellows.BP_Tool_Bellows_C" :`NewEnumerator2` "/Game/Blueprints/Player/Tools/BP_Tool_Tongs.BP_Tool_Tongs_C" :!type "Actor Class Reference")))

(event `InputAxis|UpDown`
  (params (AxisValue :type "Float (single-precision)"))
  (if (`self.IsOnReportScreen`)
    (switch `int` (`KismetMathLibrary.Round` AxisValue)
      (:`-1`
        (`/Engine/EditorBlueprintResources/StandardMacros.DoOnce` false :!label _label_6 ; Left
          (:`Completed`
            (`self.CallMenuLeft`))))
      (:`0`
        (`|ExecutionSequence`
          (:`then_0`
            (goto _label_6 :!via `Reset`))
          (:`then_1`
            (goto _label_7 :!via `Reset`))))
      (:`1`
        (`/Engine/EditorBlueprintResources/StandardMacros.DoOnce` false :!label _label_7 ; Right
          (:`Completed`
            (`self.CallMenuRight`)))))
    (else
      (`self.AddMovementInput` (1.0 0.0 0.0) AxisValue))))

(event `InputAxis|LeftRight`
  (params (AxisValue :type "Float (single-precision)"))
  (if (`self.IsOnReportScreen`)
    (switch `int` (`KismetMathLibrary.Round` AxisValue)
      (:`-1`
        (`/Engine/EditorBlueprintResources/StandardMacros.DoOnce` false :!label _label_8 ; Left
          (:`Completed`
            (`self.CallMenuLeft`))))
      (:`0`
        (`|ExecutionSequence`
          (:`then_0`
            (goto _label_8 :!via `Reset`))
          (:`then_1`
            (goto _label_9 :!via `Reset`))))
      (:`1`
        (`/Engine/EditorBlueprintResources/StandardMacros.DoOnce` false :!label _label_9 ; Right
          (:`Completed`
            (`self.CallMenuRight`)))))
    (else
      (`self.AddMovementInput` (0.0 1.0 0.0) AxisValue))))

(event `InputAction|PickUpDrop`
  (params (Key :type "Key Structure"))
  (:`Pressed`
    (if (`self.IsOnReportScreen`)
      (`self.CallMenuConfirm`))))

(fn `UserConstructionScript`)