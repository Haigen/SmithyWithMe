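; Menu player controller for local multiplayer that drives main menu navigation and lobby join/leave.
; Each controller finds its BP_LobbyActor by controller ID and toggles its joined state; controller 1 also adjusts the game mode's player count.
; Player 0 confirms or backs out via dispatchers and, once joined, starts the game after a ten-second how-to-play screen.
; DoOnce gates turn the up/down axis into single-step navigation events.
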(event `Recheck`
  (bind _outactors (`GameplayStatics.GetAllActorsOfClass` "/Game/Blueprints/Level/Lobby/BP_LobbyActor.BP_LobbyActor_C" :!label _label))
  (for _array_element _outactors
    (if (== (`/Game/Blueprints/Level/Lobby/BP_LobbyActor.ActorID` _array_element) (`GameplayStatics.GetPlayerControllerID` self))
      (set `self.LobbyActor` _array_element))))

(event `self.ReceiveBeginPlay`
  (goto _label))

(event `InputAction|PickUpDrop`
  (params (Key :type "Key Structure"))
  (bind _lobbyactor (`self.LobbyActor`))
  (bind _asbp_menu_game_mode (cast `/Game/Blueprints/BP_MenuGameMode` (`GameplayStatics.GetGameMode`) :!pure true))
  (:`Pressed`
    (if (== (`GameplayStatics.GetPlayerControllerID` self) 0)
      (if (`self.InMainMenu`)
        (`self.CallMenuConfirm`)
        (else
          (if (not (`/Game/Blueprints/Level/Lobby/BP_LobbyActor.Joined` _lobbyactor)) :!label _label_2
            (set `/Game/Blueprints/Level/Lobby/BP_LobbyActor.Joined` true _lobbyactor)
            (`/Game/Blueprints/Level/Lobby/BP_LobbyActor.UpdateJoinInfo` (`self.LobbyActor`))
            (if (== (`GameplayStatics.GetPlayerControllerID` self) 1)
              (set `/Game/Blueprints/BP_MenuGameMode.NumOfPlayers` (+ (`/Game/Blueprints/BP_MenuGameMode.NumOfPlayers` _asbp_menu_game_mode) 1) _asbp_menu_game_mode)))))
      (else
        (goto _label_2)))))

(event `InputAction|Pause`
  (params (Key :type "Key Structure"))
  (:`Pressed`
    (if (and (== (`GameplayStatics.GetPlayerControllerID` self) 0) (`/Game/Blueprints/Level/Lobby/BP_LobbyActor.Joined` (`self.LobbyActor`)))
      (bind _returnvalue (`|CreateWidget` "/Game/Blueprints/UI/WBP_HowToPlay.WBP_HowToPlay_C" self))
      (`UserWidget.AddToPlayerScreen` _returnvalue 0)
      (`KismetSystemLibrary.Delay` 10.0)
      (`/Game/Blueprints/BP_MenuGameMode.OpenLevel` (cast `/Game/Blueprints/BP_MenuGameMode` (`GameplayStatics.GetGameMode`) :!pure true)))))

(event `InputAction|Back`
  (params (Key :type "Key Structure"))
  (bind _asbp_menu_game_mode (cast `/Game/Blueprints/BP_MenuGameMode` (`GameplayStatics.GetGameMode`) :!pure true))
  (:`Pressed`
    (if (and (== (`GameplayStatics.GetPlayerControllerID` self) 0) (not (`/Game/Blueprints/Level/Lobby/BP_LobbyActor.Joined` (`self.LobbyActor`))))
      (`self.BackToMainMenu`)
      (else
        (set `/Game/Blueprints/Level/Lobby/BP_LobbyActor.Joined` false (`self.LobbyActor`))
        (`/Game/Blueprints/Level/Lobby/BP_LobbyActor.UpdateJoinInfo` (`self.LobbyActor`))
        (if (== (`GameplayStatics.GetPlayerControllerID` self) 1)
          (set `/Game/Blueprints/BP_MenuGameMode.NumOfPlayers` (- (`/Game/Blueprints/BP_MenuGameMode.NumOfPlayers` _asbp_menu_game_mode) 1) _asbp_menu_game_mode))))))

(event `InputAxis|UpDown`
  (params (AxisValue :type "Float (single-precision)"))
  (switch `int` (`KismetMathLibrary.Round` AxisValue)
    (:`-1`
      (`/Engine/EditorBlueprintResources/StandardMacros.DoOnce` false :!label _label_3 ; Down
        (:`Completed`
          (`self.MenuDown`))))
    (:`0`
      (`|ExecutionSequence`
        (:`then_0`
          (goto _label_3 :!via `Reset`))
        (:`then_1`
          (goto _label_4 :!via `Reset`))))
    (:`1`
      (`/Engine/EditorBlueprintResources/StandardMacros.DoOnce` false :!label _label_4 ; Up
        (:`Completed`
          (`self.MenuUp`))))))

(fn `UserConstructionScript`)